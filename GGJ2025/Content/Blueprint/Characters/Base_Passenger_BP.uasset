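; Base passenger Blueprint that handles a passenger's thought bubble and movement between destinations, waiting lines and seats.
; Tick turns the bubble toward the camera, wobbles it with Perlin noise and sine waves, and drags trailing dots proportionally.
; A timeline fades widget and meshes via tint and custom primitive data.
; Timeline lerps handle travel and queue offsets, MoveComponentTo handles seating, and a swept move snaps passengers to the floor.
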(event Custom|Test
  (bind _springarm (Variables|Default|GetSpringArm))
  (Utilities|FlowControl|FlipFlop
    (:A
      (Variables|/Script/Engine.SpringArmComponent|SetTargetOffset _springarm "0.000000,0.000000,200.000000"))
    (:B
      (Variables|/Script/Engine.SpringArmComponent|SetTargetOffset _springarm "0, 0, 0"))))

(event Custom|SnapOpacity
  (if (Variables|Default|GetbShowThoughts)
    (Audio|SpawnSound2D "/Game/Sounds/bubble_open.bubble_open" 1.0 1.0 0.0 0)
    (bind _opacity (Timeline|ThougthsOpacityTimeline Reverse)
      (:Update
        (CallFunction|SetThoughtsOpacity _opacity)))
    (else
      (Timeline|ThougthsOpacityTimeline Play))))

(event EventTick
  (params (DeltaSeconds :type Float%20%28single-precision%29))
  (bind _returnvalue (Utilities|Time|GetGameTimeinSeconds))
  (bind _returnvalue_2 (Game|GetPlayerCameraManager 0))
  (bind _staticmesh2 (Variables|Default|GetStaticMesh2))
  (bind _staticmesh3 (Variables|Default|GetStaticMesh3))
  (bind _staticmesh1 (Variables|Default|GetStaticMesh1))
  (bind _staticmesh (Variables|Default|GetStaticMesh))
  (bind _widget (Variables|Default|GetWidget))
  (bind _staticmesh_2 (Variables|Default|GetStaticMesh))
  (bind _returnvalue_3 (Camera|GetCameraRotation _returnvalue_2))
  (bind _array (Utilities|Array|MakeArray _staticmesh3 _staticmesh2 _staticmesh1))
  (bind _relativerotation (Variables|/Script/Engine.SceneComponent|GetRelativeRotation _widget))
  (bind _relativerotation_2 (Variables|/Script/Engine.SceneComponent|GetRelativeRotation _staticmesh_2))
  (|CallParentFunction DeltaSeconds)
  (Transformation|SetWorldRotation (Variables|Default|GetScene) (Math|Rotator|MakeRotfromXY (* (Math|Vector|GetRightVector _returnvalue_3) "-1.000000,-1.000000,-1.000000") (Math|Vector|GetForwardVector _returnvalue_3)) false false)
  (Transformation|SetRelativeRotation _widget (Math|Rotator|MakeRotator (Math|Float|MapRangeClamped (Class|KismetMathLibrary|PerlinNoise1D (* _returnvalue (Variables|Default|GetIconAngleChangeSpeed))) -1.0 1.0 -15.0 15.0) (.pitch _relativerotation) (.yaw _relativerotation)) false false)
  (Transformation|SetRelativeLocation _staticmesh_2 (Math|Vector|MakeVector 0.0 0.0 (Math|Float|MapRangeClamped (Math|Trig|Sin(Degrees) (* _returnvalue (Variables|Default|GetBubbleZBobbingSpeed))) -1.0 1.0 -5.0 5.0)) false false)
  (Transformation|SetRelativeRotation _staticmesh_2 (Math|Rotator|MakeRotator (.roll _relativerotation_2) (Math|Float|MapRangeClamped (Math|Trig|Sin(Degrees) (* (Utilities|Time|GetGameTimeinSeconds) (Variables|Default|GetBubbleRollBobbingSpeed))) -1.0 1.0 -7.5 7.5) (.yaw _relativerotation_2)) false false)
  (for (_array_element _array_index) _array
    (Transformation|SetRelativeLocation _array_element (+ (* (- (Variables|/Script/Engine.SceneComponent|GetRelativeLocation _staticmesh) (.Value (Utilities|Map|Find (Variables|Default|GetBubbleDotRelativeLocation) _staticmesh))) (/ (+ _array_index 1) (+ (Utilities|Array|Length _array) 1))) (.Value (Utilities|Map|Find (Variables|Default|GetBubbleDotRelativeLocation) _array_element))) false false)))

(event EventOnShowThoughtsStateChanged
  (if (Variables|Default|GetbShowThoughts)
    (Audio|SpawnSound2D "/Game/Sounds/bubble_open.bubble_open" 1.0 1.0 0.0 0)
    (bind _opacity (Timeline|ThougthsOpacityTimeline Reverse)
      (:Update
        (CallFunction|SetThoughtsOpacity _opacity)))
    (else
      (Timeline|ThougthsOpacityTimeline Play))))

(event EventBeginPlay
  (|CallParentFunction)
  (CallFunction|SnapOpacity)
  (for _array_element (Utilities|Array|MakeArray (Variables|Default|GetStaticMesh) (Variables|Default|GetStaticMesh2) (Variables|Default|GetStaticMesh3) (Variables|Default|GetStaticMesh1))
    (Utilities|Map|Add (Variables|Default|GetBubbleDotRelativeLocation) _array_element (Variables|/Script/Engine.SceneComponent|GetRelativeLocation _array_element))))

(event EventGotoDestination
  (params (location :type Vector%20%28by%20ref%29 :default "0, 0, 0") (rotation :type Rotator%20%28by%20ref%29 :default "0, 0, 0"))
  (bind (_x _y _z) (Math|Vector|BreakVector location))
  (bind _returnvalue (Transformation|GetActorTransform))
  (bind _mesh (Variables|Character|GetMesh))
  (bind _waitingendofline (Variables|Default|GetWaitingEndOfLine))
  (bind _relativelocation (Variables|/Script/Engine.SceneComponent|GetRelativeLocation _mesh))
  (bind _returnvalue_2 (* (.z _relativelocation) -1.0))
  (bind _output_get (Variables|Default|SetGoToOriginalLocation (.location _returnvalue)))
  (Variables|Default|SetGoToOriginalRotation (.rotation _returnvalue))
  (bind (_direction _destinationratio _zup _rotationratio) (Timeline|GoToTimeline PlayFromStart)
    (:Update
      (Transformation|SetActorLocation (Math|Vector|Lerp(Vector) (Math|Vector|Lerp(Vector) _output_get (Math|Vector|MakeVector _x _y (+ _zup _z _returnvalue_2)) (Math|Float|MapRangeClamped _destinationratio 0.0 1.0 0.0 1.0)) (+ (Math|Vector|MakeVector (.x _waitingendofline) (.y _waitingendofline) (+ (.z _waitingendofline) _returnvalue_2 _zup)) (* (Class|KismetMathLibrary|VectorNormal2D (- location (Variables|Default|GetWaitingEndOfLine)) 0.0001) (* 15 (Variables|Default|GetWaitingIndex)))) (Math|Float|MapRangeClamped _destinationratio 1.0 1.2 0.0 1.0)) false false)
      (Transformation|SetActorRotation (Math|Rotator|Lerp(Rotator) (Variables|Default|GetGoToOriginalRotation) rotation _rotationratio true)))
    (:Finished
      (CallFunction|SnaptoFloor))))

(event EventSetSeat
  (params (seat :type Train%20Seat%20Component%20Object%20Reference))
  (bind _returnvalue (Transformation|GetWorldTransform seat))
  (bind _rootcomponent (Variables|Transformation|GetRootComponent))
  (|CallParentFunction seat)
  (Utilities|IsValid seat
    (:Is%20Valid
      (Variables|Default|SetLastSeat seat))
    (:Is%20Not%20Valid
      _))
  (Utilities|IsValid seat
    (:Is%20Valid
      (Collision|SetActorEnableCollision false)
      (Utilities|FlowControl|Sequence
        (:then_0
          (goto _label_2 Stop))
        (:then_1
          (Components|MoveComponentTo _rootcomponent (.location _returnvalue) (.rotation _returnvalue) true true 0.75 false :!label _label))))
    (:Is%20Not%20Valid
      (Collision|SetActorEnableCollision true)
      (Utilities|FlowControl|Sequence
        (:then_0
          (goto _label Stop))
        (:then_1
          (Utilities|IsValid (Variables|Default|GetLastSeat)
            (:Is%20Valid
              (Components|MoveComponentTo _rootcomponent (Math|Transform|TransformLocation (Transformation|GetWorldTransform (Variables|Default|GetLastSeat)) "75.000000,0.000000,15.000000") (.Rotation (Math|Transform|BreakTransform (Transformation|GetWorldTransform (Variables|Default|GetLastSeat)))) true true 0.75 false :!label _label_2))
            (:Is%20Not%20Valid
              (Utilities|FlowControl|Delay 0.75)))
          (CallFunction|SnaptoFloor))))))

(fn ConstructionScript
  (|CallParentFunction)
  (Rendering|SetCastShadow (Variables|Default|GetWidget) false))

(fn SetThoughtsOpacity
  (params (New%20Tint%20Color%20and%20Opacity%20A :type Float%20%28single-precision%29))
  (Class|WidgetComponent|SetTintColorandOpacity (Variables|Default|GetWidget) (Utilities|Struct|MakeLinearColor 1.0 1.0 1.0 New%20Tint%20Color%20and%20Opacity%20A))
  (Rendering|Material|SetDefaultCustomPrimitiveDataFloat (Variables|Default|GetStaticMesh) 0 (- 1.0 New%20Tint%20Color%20and%20Opacity%20A)))

(fn GetSpeechText
  (return (Utilities|Text|ToText(String) (Utilities|GetObjectName self))))

(fn SnaptoFloor
  (bind _returnvalue (Transformation|GetActorLocation))
  (Transformation|SetActorLocation (+ _returnvalue "0.000000,0.000000,100.000000") false false)
  (Transformation|SetActorLocation (+ _returnvalue "0.000000,0.000000,-200.000000") true false))