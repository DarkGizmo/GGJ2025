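; Cabin actor that drives a dithered fade on its meshes based on whether a Character is inside its Box volume.
; Box begin and end overlaps both recheck overlapping Characters, playing a timeline while any is present and reversing it when none remain.
; Timeline updates write the fade alpha to custom primitive data index 0 on components tagged SupportDitherFade, presumably for their materials to read.
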(event OnComponentBeginOverlap(Box)
  (params (OverlappedComponent :type Primitive%20Component%20Object%20Reference) (OtherActor :type Actor%20Object%20Reference) (OtherComp :type Primitive%20Component%20Object%20Reference) (OtherBodyIndex :type Integer) (bFromSweep :type Boolean) (SweepResult :type Hit%20Result%20Structure%20%28by%20ref%29))
  (if (Utilities|Array|IsEmpty (Collision|GetOverlappingActors (Variables|Default|GetBox) "/Script/Engine.Character" :!class /Script/Engine.PrimitiveComponent))
    (bind _ditherfade (Timeline|Timeline Reverse)
      (:Update
        (CallFunction|SetDitheredFade _ditherfade)))
    (else
      (Timeline|Timeline Play))))

(event OnComponentEndOverlap(Box)
  (params (OverlappedComponent :type Primitive%20Component%20Object%20Reference) (OtherActor :type Actor%20Object%20Reference) (OtherComp :type Primitive%20Component%20Object%20Reference) (OtherBodyIndex :type Integer))
  (if (Utilities|Array|IsEmpty (Collision|GetOverlappingActors (Variables|Default|GetBox) "/Script/Engine.Character" :!class /Script/Engine.PrimitiveComponent))
    (bind _ditherfade (Timeline|Timeline Reverse)
      (:Update
        (CallFunction|SetDitheredFade _ditherfade)))
    (else
      (Timeline|Timeline Play))))

(event EventBeginPlay)

(event Collision|EventActorBeginOverlap
  (params (OtherActor :type Actor%20Object%20Reference)))

(event EventTick
  (params (DeltaSeconds :type Float%20%28single-precision%29)))

(fn ConstructionScript)

(fn SetDitheredFade
  (params (FadeAlpha :type Float%20%28double-precision%29))
  (for _array_element (Actor|GetComponentsByClass "/Script/Engine.PrimitiveComponent")
    (if (Components|ComponentHasTag _array_element "SupportDitherFade")
      (Rendering|Material|SetCustomPrimitiveDataFloat _array_element 0 FadeAlpha))))