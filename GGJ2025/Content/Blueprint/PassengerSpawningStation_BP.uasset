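; Station actor that spawns passengers and sends them to waiting spots in a line.
; SpawnPassengersBP spawns the requested number, gives each Passenger_BP its waiting index and the first waiting point as end of line, then calls SendPassengersToWaitingDestinations.
; The spawn and send functions are defined outside this graph.
; The construction script fills the spawning and waiting location arrays from placed point components and resets billboard relative transforms.
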(event Custom|SpawnPassengersBP
  (params (Num :type Integer))
  (for _index (range 0 (- Num 1))
    (bind _returnvalue (Class|PlayerSpawningStation|SpawnPassenger))
    (bind _aspassenger_bp (Utilities|Casting|CastToPassenger_BP _returnvalue))
    (Variables|/Game/Blueprint/Passenger_BP.Passenger_BP_C|SetWaitingIndex _aspassenger_bp _index)
    (Variables|/Game/Blueprint/Passenger_BP.Passenger_BP_C|SetWaitingEndOfLine _aspassenger_bp (Transformation|GetWorldLocation (Utilities|Array|Get(acopy) (Variables|Default|GetWaitingLocations)))))
  (Class|PlayerSpawningStation|SendPassengerstoWaitingDestinations))

(event EventBeginPlay)

(event Collision|EventActorBeginOverlap
  (params (OtherActor :type Actor%20Object%20Reference)))

(event EventTick
  (params (DeltaSeconds :type Float%20%28single-precision%29)))

(fn ConstructionScript
  (Variables|Default|SetSpawningLocations (Utilities|Array|MakeArray (Variables|Default|GetSpawnPoint01) (Variables|Default|GetSpawnPoint02) (Variables|Default|GetSpawnPoint03) (Variables|Default|GetSpawnPoint04) (Variables|Default|GetSpawnPoint05) (Variables|Default|GetSpawnPoint06) (Variables|Default|GetSpawnPoint07) (Variables|Default|GetSpawnPoint08) (Variables|Default|GetSpawnPoint09) (Variables|Default|GetSpawnPoint010) (Variables|Default|GetSpawnPoint011) (Variables|Default|GetSpawnPoint012)))
  (Variables|Default|SetWaitingLocations (Utilities|Array|MakeArray (Variables|Default|GetWaitingPoint01) (Variables|Default|GetWaitingPoint02) (Variables|Default|GetWaitingPoint03) (Variables|Default|GetWaitingPoint04) (Variables|Default|GetWaitingPoint05) (Variables|Default|GetWaitingPoint06) (Variables|Default|GetWaitingPoint07) (Variables|Default|GetWaitingPoint08) (Variables|Default|GetWaitingPoint09) (Variables|Default|GetWaitingPoint10) (Variables|Default|GetWaitingPoint11) (Variables|Default|GetWaitingPoint12)))
  (for _array_element (Actor|GetComponentsByClass "/Script/Engine.BillboardComponent")
    (Transformation|ResetRelativeTransform _array_element)))