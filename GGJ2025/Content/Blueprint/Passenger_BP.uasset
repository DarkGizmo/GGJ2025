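; Passenger Blueprint that displays an animated thought bubble, made of a widget icon and four meshes, turned toward the player camera.
; Tick wobbles the icon with Perlin noise and bobs the main bubble with sine waves, while trailing dots follow by graduated fractions from cached positions.
; ShowThoughts changes drive a timeline that fades the widget tint and the meshes through custom primitive data.
; A Test event toggles the spring arm's height offset.
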(event Custom|Test
  (bind _springarm (Variables|Default|GetSpringArm))
  (Utilities|FlowControl|FlipFlop
    (:A
      (Variables|/Script/Engine.SpringArmComponent|SetTargetOffset _springarm "0.000000,0.000000,200.000000"))
    (:B
      (Variables|/Script/Engine.SpringArmComponent|SetTargetOffset _springarm "0, 0, 0"))))

(event Custom|SnapOpacity
  (if (Variables|Default|GetbShowThoughts)
    (bind _opacity (Timeline|ThougthsOpacityTimeline Reverse)
      (:Update
        (CallFunction|SetThoughtsOpacity _opacity)))
    (else
      (Timeline|ThougthsOpacityTimeline Play))))

(event EventTick
  (params (DeltaSeconds :type Float%20%28single-precision%29))
  (bind _returnvalue (Utilities|Time|GetGameTimeinSeconds))
  (bind _returnvalue_2 (Game|GetPlayerCameraManager 0))
  (bind _staticmesh2 (Variables|Default|GetStaticMesh2))
  (bind _staticmesh3 (Variables|Default|GetStaticMesh3))
  (bind _staticmesh1 (Variables|Default|GetStaticMesh1))
  (bind _staticmesh (Variables|Default|GetStaticMesh))
  (bind _widget (Variables|Default|GetWidget))
  (bind _staticmesh_2 (Variables|Default|GetStaticMesh))
  (bind _returnvalue_3 (Camera|GetCameraRotation _returnvalue_2))
  (bind _array (Utilities|Array|MakeArray _staticmesh3 _staticmesh2 _staticmesh1))
  (bind _relativerotation (Variables|/Script/Engine.SceneComponent|GetRelativeRotation _widget))
  (bind _relativerotation_2 (Variables|/Script/Engine.SceneComponent|GetRelativeRotation _staticmesh_2))
  (|CallParentFunction DeltaSeconds)
  (Transformation|SetWorldRotation (Variables|Default|GetScene) (Math|Rotator|MakeRotfromXY (* (Math|Vector|GetRightVector _returnvalue_3) "-1.000000,-1.000000,-1.000000") (Math|Vector|GetForwardVector _returnvalue_3)) false false)
  (Transformation|SetRelativeRotation _widget (Math|Rotator|MakeRotator (Math|Float|MapRangeClamped (Class|KismetMathLibrary|PerlinNoise1D (* _returnvalue (Variables|Default|GetIconAngleChangeSpeed))) -1.0 1.0 -15.0 15.0) (.pitch _relativerotation) (.yaw _relativerotation)) false false)
  (Transformation|SetRelativeLocation _staticmesh_2 (Math|Vector|MakeVector 0.0 0.0 (Math|Float|MapRangeClamped (Math|Trig|Sin(Degrees) (* _returnvalue (Variables|Default|GetBubbleZBobbingSpeed))) -1.0 1.0 -5.0 5.0)) false false)
  (Transformation|SetRelativeRotation _staticmesh_2 (Math|Rotator|MakeRotator (.roll _relativerotation_2) (Math|Float|MapRangeClamped (Math|Trig|Sin(Degrees) (* (Utilities|Time|GetGameTimeinSeconds) (Variables|Default|GetBubbleRollBobbingSpeed))) -1.0 1.0 -7.5 7.5) (.yaw _relativerotation_2)) false false)
  (for (_array_element _array_index) _array
    (Transformation|SetRelativeLocation _array_element (+ (* (- (Variables|/Script/Engine.SceneComponent|GetRelativeLocation _staticmesh) (.Value (Utilities|Map|Find (Variables|Default|GetBubbleDotRelativeLocation) _staticmesh))) (/ (+ _array_index 1) (+ (Utilities|Array|Length _array) 1))) (.Value (Utilities|Map|Find (Variables|Default|GetBubbleDotRelativeLocation) _array_element))) false false)))

(event EventOnShowThoughtsStateChanged
  (if (Variables|Default|GetbShowThoughts)
    (bind _opacity (Timeline|ThougthsOpacityTimeline Reverse)
      (:Update
        (CallFunction|SetThoughtsOpacity _opacity)))
    (else
      (Timeline|ThougthsOpacityTimeline Play))))

(event EventBeginPlay
  (|CallParentFunction)
  (CallFunction|SnapOpacity)
  (for _array_element (Utilities|Array|MakeArray (Variables|Default|GetStaticMesh) (Variables|Default|GetStaticMesh2) (Variables|Default|GetStaticMesh3) (Variables|Default|GetStaticMesh1))
    (Utilities|Map|Add (Variables|Default|GetBubbleDotRelativeLocation) _array_element (Variables|/Script/Engine.SceneComponent|GetRelativeLocation _array_element))))

(fn ConstructionScript
  (|CallParentFunction)
  (Rendering|SetCastShadow (Variables|Default|GetWidget) false))

(fn SetThoughtsOpacity
  (params (New%20Tint%20Color%20and%20Opacity%20A :type Float%20%28single-precision%29))
  (Class|WidgetComponent|SetTintColorandOpacity (Variables|Default|GetWidget) (Utilities|Struct|MakeLinearColor 1.0 1.0 1.0 New%20Tint%20Color%20and%20Opacity%20A))
  (Rendering|Material|SetDefaultCustomPrimitiveDataFloat (Variables|Default|GetStaticMesh) 0 (- 1.0 New%20Tint%20Color%20and%20Opacity%20A)))