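; DitherTrigger_BP is a trigger volume that drives a dither fade on a set of linked actors.
; Box overlap plays a timeline forward on begin and reverses it on end, with no check on the overlapping actor.
; Each update writes the fade value to custom primitive data slot 0 on the linked actors' primitive components tagged SupportDitherFade, presumably read by their materials.
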(event OnComponentBeginOverlap(Box)
  (params (OverlappedComponent :type Primitive%20Component%20Object%20Reference) (OtherActor :type Actor%20Object%20Reference) (OtherComp :type Primitive%20Component%20Object%20Reference) (OtherBodyIndex :type Integer) (bFromSweep :type Boolean) (SweepResult :type Hit%20Result%20Structure%20%28by%20ref%29))
  (bind _ditherfade (Timeline|DitherFadeTimeline Play)
    (:Update
      (CallFunction|SetDitheredFade _ditherfade))))

(event OnComponentEndOverlap(Box)
  (params (OverlappedComponent :type Primitive%20Component%20Object%20Reference) (OtherActor :type Actor%20Object%20Reference) (OtherComp :type Primitive%20Component%20Object%20Reference) (OtherBodyIndex :type Integer))
  (bind _ditherfade (Timeline|DitherFadeTimeline Reverse)
    (:Update
      (CallFunction|SetDitheredFade _ditherfade))))

(fn ConstructionScript)

(fn SetDitheredFade
  (params (FadeAlpha :type Float%20%28double-precision%29))
  (for _array_element (Variables|Default|GetLinkedActors)
    (for _array_element_2 (Actor|GetComponentsByClass _array_element "/Script/Engine.PrimitiveComponent")
      (if (Components|ComponentHasTag _array_element_2 "SupportDitherFade")
        (Rendering|Material|SetCustomPrimitiveDataFloat _array_element_2 0 FadeAlpha)))))