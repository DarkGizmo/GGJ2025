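; Interaction component for the departure bell that lets a character ring it to notify the game mode.
; It caches BP_GGJGameMode2025 on BeginPlay and is interactible only while that game mode reports the bell can be rung.
; Interacting calls RingBell on the game mode and plays the departure bell sound in 2D.
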(event EventBeginPlay
  (|CallParentFunction)
  (bind _asbp_ggjgame_mode_2025 (Utilities|Casting|CastToBP_GGJGameMode2025 (Game|GetGameMode)))
  (Variables|Default|SetGameMode _asbp_ggjgame_mode_2025))

(event EventOnInteract
  (params (character :type GGJ2025%20Character%20Object%20Reference))
  (Class|GGJ2025GameMode|RingBell (Variables|Default|GetGameMode))
  (Audio|SpawnSound2D "/Game/Sounds/departure_bell.departure_bell" 1.0 1.0 0.0 0))

(fn IsInteractible
  (params (character :type GGJ2025%20Character%20Object%20Reference))
  (bind _gamemode (Variables|Default|GetGameMode))
  (Utilities|IsValid _gamemode
    (:Is%20Valid
      (return (Class|GGJ2025GameMode|CanBellbeRung _gamemode)))
    (:Is%20Not%20Valid
      (return false))))