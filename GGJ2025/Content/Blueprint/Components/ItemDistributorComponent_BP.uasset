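; Interactible component that hands out an item of a configured class to the character who interacts with it.
; It only gives the item, shows its take-item prompt and reports itself interactible while that character's hands are empty.
; With no held item, the interactibility check defers to the parent component's rule; otherwise it returns false and the prompt text is blank.
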(event EventOnInteract
  (params (character :type GGJ2025%20Character%20Object%20Reference))
  (Utilities|IsValid (Variables|/Script/GGJ2025.GGJ2025Character|GetHeldItem character)
    (:Is%20Not%20Valid
      (Class|GGJ2025Character|GiveItem character (Variables|Default|GetItemClass)))))

(fn GetInteractText
  (params (character :type GGJ2025%20Character%20Object%20Reference))
  (Utilities|IsValid (Variables|/Script/GGJ2025.GGJ2025Character|GetHeldItem character)
    (:Is%20Valid
      (return ""))
    (:Is%20Not%20Valid
      (return (Variables|Default|GetTakeItemText)))))

(fn IsInteractible
  (params (character :type GGJ2025%20Character%20Object%20Reference))
  (Utilities|IsValid (Variables|/Script/GGJ2025.GGJ2025Character|GetHeldItem character)
    (:Is%20Valid
      (return false))
    (:Is%20Not%20Valid
      (return (|CallParentFunction 0)))))