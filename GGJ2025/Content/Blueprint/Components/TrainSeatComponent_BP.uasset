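; TrainSeatComponent_BP is a train seat component that shows a seat selector world UI while the seat is in focus.
; On a focus change it destroys any existing widget actor and clears the reference.
; When focus is gained it then spawns a new SeatSelector_WorldUI_BP at an offset above the component's world transform and stores it for later cleanup.
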(event EventInFocusChanged
  (params (bInFocus :type Boolean))
  (if bInFocus
    (Utilities|FlowControl|Sequence
      (:then_0
        (Utilities|IsValid (Variables|Default|GetWidget) :!label _label
          (:Is%20Valid
            (Actor|DestroyActor (Variables|Default|GetWidget))
            (Variables|Default|SetWidget 0))))
      (:then_1
        (bind _returnvalue (Game|SpawnActorfromClass "/Game/Blueprint/SeatSelector_WorldUI_BP.SeatSelector_WorldUI_BP_C" (Math|Transform|ComposeTransforms (Transformation|GetWorldTransform) (Math|Transform|MakeTransform "0.000000,0.000000,20.000000")) "AlwaysSpawn" "MultiplyWithRoot" 0 0))
        (Variables|Default|SetWidget _returnvalue)))
    (else
      (goto _label))))