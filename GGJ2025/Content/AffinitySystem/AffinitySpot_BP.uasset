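; AffinitySpot is an actor component marking a spot that holds an assigned actor and scores how well it suits its surroundings.
; GetScore sums that actor's Affinities values matching the Characteristics of the spot and of actors assigned to neighbouring spots, both read through Characteristics_BP.
; It returns zero without a valid actor or neighbours, logging the latter.
; With DebugDraw on, Tick draws neighbour arrows and the score, coloured by whether it is positive.
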(event EventBeginPlay)

(event EventTick
  (params (DeltaSeconds :type Float%20%28single-precision%29))
  (if (Variables|Default|GetDebugDraw)
    (Utilities|FlowControl|Sequence
      (:then_0
        ;[0.15 0.15 0.15 0.5] Draw debug neighbour links
        (for _array_element (Variables|Default|GetNeighbours)
          (Rendering|Debug|DrawDebugArrow (Transformation|GetActorLocation (Components|GetOwner)) (Transformation|GetActorLocation _array_element) 1e+01 (Math|Color|MakeColor 0.0 0.0 1.0) 0.0 1e+01)))
      (:then_1
        (bind _score (CallFunction|GetScore))
        (Rendering|Debug|DrawDebugString "0, 0, 0" (Utilities|String|ToString(Integer) _score) (Components|GetOwner) (Math|Color|SelectColor "(R=0.000000,G=0.630208,B=0.141719,A=1.000000)" "(R=1.000000,G=0.000000,B=0.000000,A=1.000000)" (> _score 0)))))))

(fn AssignActor
  (params (actor :type Actor%20Object%20Reference))
  (Variables|Default|SetAssignedActor actor))

(fn GetScore
  (LocalVariables|SetresultScore 0)
  (Utilities|IsValid (Variables|Default|GetAssignedActor)
    (:Is%20Valid
      (if (Utilities|Array|IsNotEmpty (Variables|Default|GetNeighbours))
        (Utilities|FlowControl|Sequence
          (:then_0
            ;[0.15 0.15 0.15 0.5] For each neighbour
            (for _array_element (Variables|Default|GetNeighbours)
              ;[0.15 0.15 0.15 0.5] For each characteristics
              (for _array_element_2 (Variables|/Game/AffinitySystem/Characteristics_BP.Characteristics_BP_C|GetCharacteristics (Actor|GetComponentbyClass (Variables|AffinitySpot_BP_C|GetAssignedActor (Actor|GetComponentbyClass _array_element "AffinitySpot_BP_C")) "/Game/AffinitySystem/Characteristics_BP.Characteristics_BP_C"))
                (if (.ReturnValue (Utilities|Map|Find (Variables|/Game/AffinitySystem/Characteristics_BP.Characteristics_BP_C|GetAffinities (Actor|GetComponentbyClass (Variables|Default|GetAssignedActor) "/Game/AffinitySystem/Characteristics_BP.Characteristics_BP_C")) _array_element_2))
                  ;[0.15 0.15 0.15 0.5] Add to the score to the result
                  (LocalVariables|SetresultScore (+ (.Value (Utilities|Map|Find (Variables|/Game/AffinitySystem/Characteristics_BP.Characteristics_BP_C|GetAffinities (Actor|GetComponentbyClass (Variables|Default|GetAssignedActor) "/Game/AffinitySystem/Characteristics_BP.Characteristics_BP_C")) _array_element_2)) (LocalVariables|GetresultScore)))))))
          (:then_1
            ;[0.15 0.15 0.15 0.5] For each characteristics of this spot
            (for _array_element_3 (Variables|Default|GetCharacteristics)
              (if (.ReturnValue (Utilities|Map|Find (Variables|/Game/AffinitySystem/Characteristics_BP.Characteristics_BP_C|GetAffinities (Actor|GetComponentbyClass (Variables|Default|GetAssignedActor) "/Game/AffinitySystem/Characteristics_BP.Characteristics_BP_C")) _array_element_3))
                ;[0.15 0.15 0.15 0.5] Add to the score to the result
                (LocalVariables|SetresultScore (+ (.Value (Utilities|Map|Find (Variables|/Game/AffinitySystem/Characteristics_BP.Characteristics_BP_C|GetAffinities (Actor|GetComponentbyClass (Variables|Default|GetAssignedActor) "/Game/AffinitySystem/Characteristics_BP.Characteristics_BP_C")) _array_element_3)) (LocalVariables|GetresultScore))))))
          (:then_2
            (return (LocalVariables|GetresultScore))))
        (else
          (Utilities|String|LogString (Utilities|String|Append "Invalid AffinitySpot has no neighbours: " (Class|KismetSystemLibrary|GetPathName self)))
          (return 0))))
    (:Is%20Not%20Valid
      (return 0))))